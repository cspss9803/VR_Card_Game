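; BP_NPC_Display is a display NPC that shows a chosen NPC type with a buff list widget above its head.
; BeginPlay picks the skeletal mesh and color by type, creates WB_BuffList, and plays a timeline-driven dissolve on material and Niagara particles in that color.
; An event passes new buffs to the widget to reset its list.
; Tick turns the widget toward the owning player controller's camera.
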(event Custom|將新的%20Buff%20加到樣本角色頭上的介面
  (params (Buff :type E_Buff%20Enum :default "NewEnumerator4"))
  (bind _aswb_buff_list (Utilities|Casting|CastToWB_BuffList (UserInterface|GetWidget (Variables|Default|GetWidget))))
  (Default|ResetBuffList _aswb_buff_list Buff))

(event EventBeginPlay
  (bind _npc_種類 (Variables|Default|GetNPC%20種類))
  (bind _niagarasystemdissolving (Variables|Default|GetNiagaraSystemDissolving))
  (bind _mesh (Variables|Character|GetMesh))
  (bind _顏色 (CallFunction|取得NPC的顏色 _npc_種類))
  (bind _returnvalue (Math|Conversions|ToVector(LinearColor) _顏色))
  (Components|SkeletalMesh|SetSkeletalMeshAsset (Variables|Character|GetMesh) (CallFunction|取得NPC的骨骼模型 (Variables|Default|GetNPC%20種類)))
  (Utilities|FlowControl|Sequence
    (:then_0
      (Class|WidgetComponent|SetDrawSize (Variables|Default|GetWidget) "(X=1500.000000,Y=300.000000)")
      (bind _returnvalue_2 (UserInterface|CreateWidget "/Game/_CardGame/3D_介面/MainMap/BuffList/WB_BuffList.WB_BuffList_C" 0 self))
      (UserInterface|SetWidget (Variables|Default|GetWidget) _returnvalue_2))
    (:then_1
      (Rendering|Material|SetVectorParameterValueonMaterials (Variables|Character|GetMesh) "Tint" _returnvalue)
      (Utilities|FlowControl|Sequence
        (:then_0
          (Rendering|Material|SetScalarParameterValueonMaterials _mesh "DissolvingAmount" 1.0)
          (Niagara|SetNiagaraVariable(Float) _niagarasystemdissolving "DissolvingAmount" 1.0)
          (bind _tl_animation (Timeline|Timeline Play)
            (:Update
              (Rendering|Material|SetScalarParameterValueonMaterials (Variables|Character|GetMesh) "DissolvingAmount" _tl_animation)
              (Niagara|SetNiagaraVariable(Float) (Variables|Default|GetNiagaraSystemDissolving) "DissolvingAmount" _tl_animation))))
        (:then_1
          (Rendering|Material|SetVectorParameterValueonMaterials _mesh "DissolvingEdgeColor" _returnvalue)
          (Niagara|SetNiagaraVariable(LinearColor) _niagarasystemdissolving "ParitcleColor" _顏色))))))

(event EventTick
  (params (DeltaSeconds :type Float%20%28single-precision%29))
  (bind _widget (Variables|Default|GetWidget))
  (bind _asplayer_controller (Utilities|Casting|CastToPlayerController (Components|GetOwner)))
  (Transformation|SetWorldRotation _widget (Math|Rotator|FindLookatRotation (Transformation|GetWorldLocation _widget) (Camera|GetCameraLocation (Variables|/Script/Engine.PlayerController|GetPlayerCameraManager _asplayer_controller))) false false) ; 設定 Widget 的旋轉值，讓它面向鏡頭
)

(fn ConstructionScript)

(fn 取得NPC的骨骼模型
  (params (NPC :type E_Character%20Enum :default "NewEnumerator0"))
  (switch Utilities|FlowControl|Switch|SwitchonE_Character NPC
    (:NewEnumerator0
      (return 0))
    (:NewEnumerator4
      (return "/Game/_AI/NPC_Lava/素材/lava_Golem_low_1.lava_Golem_low_1"))
    (:NewEnumerator5
      (return "/Game/_AI/NPC_Man/素材/Peasant_Man.Peasant_Man"))
    (:NewEnumerator6
      (return "/Game/_AI/NPC_S_Goblin/素材/Low_Mesh_Rig.Low_Mesh_Rig"))
    (:NewEnumerator7
      (return "/Game/_AI/NPC_Mutant/素材/Mutant.Mutant"))
    (:NewEnumerator8
      (return "/Game/_AI/NPC_Goblin/素材/G_R_1.G_R_1"))
    (:NewEnumerator9
      (return "/Game/_AI/NPC_Forest/素材/R1.R1"))
    (:NewEnumerator10
      (return "/Game/_AI/NPC_Beast/素材/beast_RIG.beast_RIG"))
    (:NewEnumerator11
      (return "/Game/_AI/NPC_SpearMan/素材/Man_Rig.Man_Rig"))
    (:NewEnumerator12
      (return "/Game/_AI/NPC_Human/素材/Human_R.Human_R"))))