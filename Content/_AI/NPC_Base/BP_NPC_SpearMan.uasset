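; Spear-wielding NPC child Blueprint that specializes its parent with weapon-specific attack montages and transforms.
; On BeginPlay it assigns a spear combo as the normal attack and a Twinblades montage as the advanced attack, then calls the parent.
; F_WeaponTransform converts the weapon mesh's hand_l socket location into RightHand bone space, with zero rotation and unit scale.
; F_Get發射位置 returns the weapon's launch-position socket transform in world space.
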(event EventBeginPlay
  (Variables|Default|Set普通攻擊_Montage "/Game/_AI/NPC_SpearMan/動作/Frank_RPG_Spear_Combo05_1_Montage.Frank_RPG_Spear_Combo05_1_Montage")
  (Variables|Default|Set進階攻擊_Montage "/Game/_AI/NPC_SpearMan/動作/Twinblades_Attack19_Montage.Twinblades_Attack19_Montage")
  (|CallParentFunction))

(event Collision|EventActorBeginOverlap
  (params (OtherActor :type Actor%20Object%20Reference)))

(event EventTick
  (params (DeltaSeconds :type Float%20%28single-precision%29)))

(fn ConstructionScript
  (|CallParentFunction))

(fn FWeaponTransform
  (bind _staticmesh (Variables|Default|GetStaticMesh))
  (Utilities|IsValid _staticmesh
    (:Is%20Valid
      (return (Math|Transform|MakeTransform (.OutPosition (Class|SkinnedMeshComponent|TransformtoBoneSpace (Variables|Character|GetMesh) "RightHand" (.location (Transformation|GetSocketTransform _staticmesh "hand_l" "RTS_World")) "0, 0, 0")) "0, 0, 0" "1.000000,1.000000,1.000000")))))

(fn FGet發射位置
  (bind _staticmesh (Variables|Default|GetStaticMesh))
  (Utilities|IsValid _staticmesh
    (:Is%20Valid
      (return (Transformation|GetSocketTransform _staticmesh "發射位置" "RTS_World")))))