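; BP_R is a character with two key-triggered skills: a goblin summon and a health buff.
; Key 2 spends mana (魔力值), locks movement and recasting, and plays cast montages, with a notify starting 召喚.
; The summon picks spawn offsets by yaw quadrant, using looping DoN nodes to spawn up to three BP_S_Goblins in sequence after vortex effects.
; Key 3 triggers BP_Buff_增加生命 at the root, whose overlap callback only prints actor names.
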(event Custom|HealthActor
  (params (Actor :type Actor%20Object%20Reference))
  (Development|PrintString (Utilities|GetDisplayName Actor)))

(event Custom|召喚
  (|CollapseGraph))

(event Input|KeyboardEvents|2
  (params (Key :type Key%20Structure))
  (bind _charactermovement (Variables|Character|GetCharacterMovement))
  (:Pressed
    (if (>= (Variables|Default|Get魔力值) 2e+01)
      (if (Variables|Default|Get是否可以再次攻擊?)
        (Variables|Default|Set是否可以再次攻擊? false)
        (Variables|Default|Set魔力值 (- (Variables|Default|Get魔力值) 2e+01))
        (Components|Activation|SetActive _charactermovement false false)
        (bind _notifyname (Animation|Montage|PlayMontage (Variables|Character|GetMesh) "/Game/_AI/NPC_Forest/動作/Attack_09_Begin_Seq_Montage.Attack_09_Begin_Seq_Montage")
          (:OnNotifyBegin
            (switch name _notifyname
              (:Attack
                (Animation|Montage|PlayMontage (Variables|Character|GetMesh) "/Game/_AI/NPC_Forest/動作/Attack_09_Loop_Seq_Montage.Attack_09_Loop_Seq_Montage" 0.5
                  (:then
                    (CallFunction|召喚))
                  (:OnCompleted
                    (Components|Activation|SetActive _charactermovement true false)
                    (Variables|Default|Set是否可以再次攻擊? true)
                    (CallFunction|再次使用)))))))))))

(event Input|KeyboardEvents|3
  (params (Key :type Key%20Structure))
  (bind _mesh (Variables|Character|GetMesh))
  (:Pressed
    (bind _returnvalue (Game|SpawnActorfromClass "/Game/_Attack/BUFF/BP_Buff_增加生命.BP_Buff_增加生命_C" (Math|Transform|MakeTransform (Transformation|GetSocketLocation _mesh (Class|SkinnedMeshComponent|GetSocketBoneName _mesh "Root")) "0, 0, 0" "1.000000,1.000000,1.000000") "Undefined" self 0))
    (EventDispatchers|BindEventtoOnBuffOverlapActor _returnvalue (delegate Custom|HealthActor))
    (Default|Trigger _returnvalue)))

(fn ConstructionScript)

(event Custom|再次使用
  (bind _self self)
  (bind _spawn_transform_location (Variables|Default|GetSpawn%20Transform%20Location))
  (bind _returnvalue (Transformation|GetActorRotation _self))
  (switch int (Variables|Default|Get位置)
    (:1
      (Utilities|FlowControl|DoN 3) ; enters at Reset
    )
    (:2
      (Utilities|FlowControl|DoN 3) ; enters at Reset
    )
    (:3
      (Utilities|FlowControl|DoN 3) ; enters at Reset
    )
    (:4
      (Utilities|FlowControl|DoN 3) ; enters at Reset
    )))