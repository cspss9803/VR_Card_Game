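; Forest NPC Blueprint that adds a colored weapon dissolve effect on top of its parent NPC class when play begins.
; After parent BeginPlay, a timeline (武器消散, weapon dissipation) drives DissolvingAmount from an initial full value on both the static mesh materials and a Niagara system.
; An HDR orange-red color, set before the parent call, tints both the dissolve edge and the particles.
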(event EventBeginPlay
  (bind _staticmesh (Variables|Default|GetStaticMesh))
  (bind _niagarasmdissolving (Variables|Default|GetNiagaraSMDissolving))
  (bind _output_get (Variables|Default|Set顏色 "(R=10.000000,G=0.824327,B=0.000000,A=1.000000)"))
  (|CallParentFunction)
  (Utilities|FlowControl|Sequence
    (:then_0
      (Rendering|Material|SetScalarParameterValueonMaterials _staticmesh "DissolvingAmount" 1.0)
      (Niagara|SetNiagaraVariable(Float) _niagarasmdissolving "DissolvingAmount" 1.0)
      (bind _tl_animation (Timeline|Timeline_武器消散 Play)
        (:Update
          (Rendering|Material|SetScalarParameterValueonMaterials (Variables|Default|GetStaticMesh) "DissolvingAmount" _tl_animation)
          (Niagara|SetNiagaraVariable(Float) (Variables|Default|GetNiagaraSMDissolving) "DissolvingAmount" _tl_animation))))
    (:then_1
      (Rendering|Material|SetVectorParameterValueonMaterials _staticmesh "DissolvingEdgeColor" (Math|Conversions|ToVector(LinearColor) _output_get))
      (Niagara|SetNiagaraVariable(LinearColor) _niagarasmdissolving "ParticleColor" (Math|Conversions|ToLinearColor(Vector) (Math|Conversions|ToVector(LinearColor) _output_get))))))

(fn ConstructionScript
  (|CallParentFunction))