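; Base area-of-effect attack actor that detects pawns and reports them through event dispatchers, leaving the response to listeners.
; Trigger runs a sphere overlap at the actor's location with a configurable radius and broadcasts OnAOEOverlapActor for each pawn found.
; A separate HitActor event sweeps a fixed-size debug-drawn sphere trace forward and broadcasts OnAOEHitActor for the hit actor.
; Both queries can optionally ignore the instigator.
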(event Custom|SpawnAOE
  (bind _outactors (Collision|SphereOverlapActors (Transformation|GetActorLocation) (Variables|Default|GetSphere%20Radius) (Utilities|Array|MakeArray "ObjectTypeQuery3") 0 (select (Variables|Default|GetIgnore%20Instigator) (Utilities|Array|MakeArray (Game|GetInstigator)) 0)))
  (for _array_element _outactors
    (Default|CallOnAOEOverlapActor _array_element)))

(event Custom|Trigger
  (CallFunction|SpawnAOE))

(event Custom|HitActor
  (bind _returnvalue (Transformation|GetActorLocation))
  (bind (_outhit _returnvalue_2) (Collision|SphereTraceForObjects _returnvalue (+ _returnvalue (* (Transformation|GetActorForwardVector) 2.5e+02)) 2e+02 (Utilities|Array|MakeArray "ObjectTypeQuery3") false (select (Variables|Default|GetIgnore%20Instigator) (Utilities|Array|MakeArray (Game|GetInstigator)) 0) "ForDuration"))
  (if _returnvalue_2
    (Default|CallOnAOEHitActor (.HitActor (Collision|BreakHitResult _outhit)))))

(fn ConstructionScript)