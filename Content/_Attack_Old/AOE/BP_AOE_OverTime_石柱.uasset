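; Stone pillar (石柱) area-of-effect-over-time attack that adds a rock particle effect to the behavior inherited from its parent.
; HitActor and Trigger each call the parent, then 生成特效 (spawn effect).
; That event routes through a server event when remote, then a multicast that attaches the P_ky_rock2 emitter to the root.
; Niagara strike and sound nodes are left unconnected and never run.
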(event Custom|生成特效
  (Networking|SwitchHasAuthority
    (:Authority
      (CallFunction|生成特效Multicast))
    (:Remote
      (CallFunction|生成特效Server))))

(event Custom|生成特效_Server
  (CallFunction|生成特效Multicast))

(event Custom|生成特效_Multicast
  (Effects|SpawnEmitterAttached "/Game/_AI_Old/NPC_Beast/特效/AdvancedMagicFX11/Particles/P_ky_rock2.P_ky_rock2" (Variables|Default|GetDefaultSceneRoot) "None"))

(event EventBeginPlay
  (|CallParentFunction) ; This node is disabled and will not be called.\nDrag off pins to build functionality.
)

(event Collision|EventActorBeginOverlap
  (params (OtherActor :type Actor%20Object%20Reference))
  (|CallParentFunction OtherActor) ; This node is disabled and will not be called.\nDrag off pins to build functionality.
)

(event EventTick
  (params (DeltaSeconds :type Float%20%28single-precision%29))
  (|CallParentFunction DeltaSeconds) ; This node is disabled and will not be called.\nDrag off pins to build functionality.
)

(event EventTrigger
  (|CallParentFunction)
  (CallFunction|生成特效))

(event EventHitActor
  (|CallParentFunction)
  (CallFunction|生成特效))

(fn ConstructionScript
  (|CallParentFunction))