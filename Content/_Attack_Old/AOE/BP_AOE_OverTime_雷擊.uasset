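; Lightning strike (雷击) variant of an over-time AOE attack actor, adding the strike's visual and sound effects on top of its parent's logic.
; Trigger calls the parent, then 生成特效 (spawn effects), which multicasts directly on authority or routes through a server event otherwise.
; The multicast attaches the NS_PurpleStrike Niagara system to the root and plays a sound at the actor's location.
; A dust emitter spawn is left unconnected.
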(event Custom|生成特效
  (Networking|SwitchHasAuthority
    (:Authority
      (CallFunction|生成特效Multicast))
    (:Remote
      (CallFunction|生成特效Server))))

(event Custom|生成特效_Server
  (CallFunction|生成特效Multicast))

(event Custom|生成特效_Multicast
  (Niagara|SpawnSystemAttached "/Game/_AI_Old/NPC_Goblin/特效/StylizedVFX-AirStrikes/Particles/NS_PurpleStrike.NS_PurpleStrike" (Variables|Default|GetDefaultSceneRoot) "None" "0, 0, 0" "0, 0, 0" "KeepRelativeOffset" false)
  (Audio|PlaySoundatLocation "/Game/_AI_Old/NPC_Goblin/音效/第二招音效.第二招音效" (Transformation|GetActorLocation self) "0, 0, 0" 1.0 1.0 0.0 0 0 0 0))

(event EventBeginPlay
  (|CallParentFunction) ; This node is disabled and will not be called.\nDrag off pins to build functionality.
)

(event Collision|EventActorBeginOverlap
  (params (OtherActor :type Actor%20Object%20Reference))
  (|CallParentFunction OtherActor) ; This node is disabled and will not be called.\nDrag off pins to build functionality.
)

(event EventTick
  (params (DeltaSeconds :type Float%20%28single-precision%29))
  (|CallParentFunction DeltaSeconds) ; This node is disabled and will not be called.\nDrag off pins to build functionality.
)

(event EventTrigger
  (|CallParentFunction)
  (CallFunction|生成特效))

(fn ConstructionScript
  (|CallParentFunction))