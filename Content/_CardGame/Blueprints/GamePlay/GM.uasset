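; GameMode for a two-player VR card game that handles logins, team setup and the start of the match.
; Construction randomizes Red/Blue team order, and PostLogin registers each player, makes any extra player leave, and advances GameState's stage to character arrangement once two have joined.
; Each player gets a possessed VR pawn at team spawn markers, which are destroyed after use, a PlayerState team and a mirrored row of life crystals.
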(event EventPostLogin
  (params (NewPlayer :type Player%20Controller%20Object%20Reference))
  (|儲存剛登入的玩家 NewPlayer)
  (Utilities|玩家到齊了嗎?
    (:已經到齊
      (|踢出多餘的玩家))
    (:尚未到齊
      (|把新玩家加入玩家名單中)
      (CallFunction|創建角色與生命水晶並設定陣營)
      (|更新玩家列表介面)
      (Utilities|玩家到齊了嗎?
        (:已經到齊
          (|進入對戰角色案排階段))))))

(fn ConstructionScript
  (bind _陣營分配列表 (Variables|Default|Get陣營分配列表))
  (bind _陣營分配列表_2 (Variables|Default|Get陣營分配列表))
  (switch int (Math|Random|RandomInteger 2)
    (:0
      (Utilities|Array|Add _陣營分配列表_2 "NewEnumerator1")
      (Utilities|Array|Add _陣營分配列表_2 "NewEnumerator2"))
    (:1
      (Utilities|Array|Add _陣營分配列表 "NewEnumerator2")
      (Utilities|Array|Add _陣營分配列表 "NewEnumerator1"))))

(fn 創建角色與生命水晶並設定陣營
  (LocalVariables|Set玩家編號 (Utilities|Array|FindItem (Variables|Default|Get玩家名單PC) (Variables|Default|Get剛登入的玩家)))
  (LocalVariables|Set玩家陣營 (Utilities|Array|Get(acopy) (Variables|Default|Get陣營分配列表) (LocalVariables|Get玩家編號)))
  (switch int (LocalVariables|Get玩家編號)
    (:0
      (LocalVariables|Set是否是監聽伺服器的主人? (not (Networking|IsDedicatedServer))))
    (:1
      _))
  (Utilities|FlowControl|Sequence
    (:then_0
      ;[1 1 1] 生成玩家角色
      (switch Utilities|FlowControl|Switch|SwitchonE_Team (LocalVariables|Get玩家陣營)
        (:NewEnumerator1
          (bind _returnvalue (Actor|GetActorOfClass "/Game/_CardGame/Blueprints/SpawnPoints/Player/Actor_Player_SpawnPoint_Red.Actor_Player_SpawnPoint_Red_C"))
          (LocalVariables|Set玩家出生點 (Transformation|GetActorTransform _returnvalue))
          (Actor|DestroyActor _returnvalue)
          (bind _returnvalue_2 (Actor|GetActorOfClass "/Game/_CardGame/Blueprints/SpawnPoints/CardSlot/Actor_CardSlot0_SpawnPoint_Red.Actor_CardSlot0_SpawnPoint_Red_C"))
          (LocalVariables|Set角色安排槽位生成基點 (Transformation|GetActorTransform _returnvalue_2))
          (Actor|DestroyActor _returnvalue_2))
        (:NewEnumerator2
          (bind _returnvalue_3 (Actor|GetActorOfClass "/Game/_CardGame/Blueprints/SpawnPoints/Player/Actor_Player_SpawnPoint_Blue.Actor_Player_SpawnPoint_Blue_C"))
          (LocalVariables|Set玩家出生點 (Transformation|GetActorTransform _returnvalue_3))
          (Actor|DestroyActor _returnvalue_3)
          (bind _returnvalue_4 (Actor|GetActorOfClass "/Game/_CardGame/Blueprints/SpawnPoints/CardSlot/Actor_CardSlot0_SpawnPoint_Blue.Actor_CardSlot0_SpawnPoint_Blue_C"))
          (LocalVariables|Set角色安排槽位生成基點 (Transformation|GetActorTransform _returnvalue_4))
          (Actor|DestroyActor _returnvalue_4)))
      (bind _returnvalue_5 (Game|SpawnActorfromClass "/Game/_CardGame/Blueprints/VRPawn_Main.VRPawn_Main_C" (LocalVariables|Get玩家出生點) "Undefined" (Variables|Default|Get剛登入的玩家) (LocalVariables|Get玩家陣營) (LocalVariables|Get玩家編號) (LocalVariables|Get是否是監聽伺服器的主人?) (.Location (Math|Transform|BreakTransform (LocalVariables|Get玩家出生點))) (LocalVariables|Get角色安排槽位生成基點) 0))
      (Pawn|Possess (Variables|Default|Get剛登入的玩家) _returnvalue_5))
    (:then_1
      ;[1 1 1] 把隊伍資料存進 PlayerState
      (bind _asps (Utilities|Casting|CastToPS (Variables|/Script/Engine.Controller|GetPlayerState (Variables|Default|Get剛登入的玩家))))
      (Variables|/Game/_CardGame/Blueprints/GamePlay/PS.PS_C|SetTeam _asps (LocalVariables|Get玩家陣營)))
    (:then_2
      ;[1 1 1] 生成生命水晶
      (for _index (range 0 2)
        (bind _水晶生成位置 (CallFunction|計算生命水晶的生成位置 (LocalVariables|Get玩家陣營) _index 6e+01))
        (Game|SpawnActorfromClass "/Game/_CardGame/Blueprints/BP_Crystal.BP_Crystal_C" _水晶生成位置 "Undefined" (Variables|Default|Get剛登入的玩家) _index (LocalVariables|Get玩家陣營) 0)))))

(fn 計算生命水晶的生成位置
  (params (水晶隸屬陣營 :type E_Team%20Enum :default "NewEnumerator0") (水晶編號 :type Integer) (水晶間距 :type Float%20%28double-precision%29))
  (LocalVariables|Set間距 水晶間距)
  (switch Utilities|FlowControl|Switch|SwitchonE_Team 水晶隸屬陣營
    (:NewEnumerator1
      (LocalVariables|Set間距 (* (LocalVariables|Get間距) -1.0))
      (bind _returnvalue (Actor|GetActorOfClass "/Game/_CardGame/Blueprints/SpawnPoints/Crystal/BP_Crystal_SpawnPoints_Red.BP_Crystal_SpawnPoints_Red_C"))
      (LocalVariables|Set水晶生成基點 (Transformation|GetActorTransform _returnvalue)))
    (:NewEnumerator2
      (LocalVariables|Set間距 (* (LocalVariables|Get間距) 1.0))
      (bind _returnvalue_2 (Actor|GetActorOfClass "/Game/_CardGame/Blueprints/SpawnPoints/Crystal/BP_Crystal_SpawnPoints_Blue.BP_Crystal_SpawnPoints_Blue_C"))
      (LocalVariables|Set水晶生成基點 (Transformation|GetActorTransform _returnvalue_2))))
  (return (Math|Transform|MakeTransform (Math|Vector|MakeVector (.X (Class|KismetMathLibrary|BreakVector3f (.Location (Math|Transform|BreakTransform (LocalVariables|Get水晶生成基點))))) (+ (.Y (Class|KismetMathLibrary|BreakVector3f (.Location (Math|Transform|BreakTransform (LocalVariables|Get水晶生成基點))))) (* 水晶編號 (LocalVariables|Get間距))) (.Z (Class|KismetMathLibrary|BreakVector3f (.Location (Math|Transform|BreakTransform (LocalVariables|Get水晶生成基點)))))) (.Rotation (Math|Transform|BreakTransform (LocalVariables|Get水晶生成基點))) (.Scale (Math|Transform|BreakTransform (LocalVariables|Get水晶生成基點))))))