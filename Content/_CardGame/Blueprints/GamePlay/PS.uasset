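; PlayerState for a team card-battle game, holding each player's name, battle score and queue of battle characters.
; BeginPlay polls each tick until a team is assigned to cache its spawn transform, and passes the GameInstance name to the server via RPCs.
; SpawnBattleCharacter spawns and dequeues the first BattleList entry.
; RepNotifies refresh the 3D player list; a nonzero score also destroys remaining NPCs and sets GameStage on the server.
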(event EventBeginPlay
  (Utilities|FlowControl|Sequence
    (:then_0
      (|儲存對戰角色的生成位置))
    (:then_1
      (|把GameInstance中儲存的玩家名稱儲存到PlayerState))))

(fn ConstructionScript)

(fn OnRepBattleScore
  (|是否要進行重置
    (:更新記分板就好
      (|更新記分板 :!label _label))
    (:重置
      (Utilities|FlowControl|Sequence
        (:then_0
          (goto _label))
        (:then_1
          (|清除戰鬥結束後還留在場上的所有對戰角色))
        (:then_2
          (|檢查是否滿足勝利條件))))))

(fn OnRepUserName
  (bind _returnvalue (Actor|GetActorOfClass "/Game/_CardGame/3D_Widget/MainMap/PlayerList/Actor_3D_Widget_PlayerList.Actor_3D_Widget_PlayerList_C"))
  (Default|UpdatePlayerList _returnvalue))

(event Custom|setName_RunOnServer
  (params (UserName :type Text))
  (Variables|Default|SetUserName UserName))

(event Custom|GetPlayerName_RunOnOwningClient
  (bind _gi (CallFunction|GetGI))
  (bind _playername (Variables|/Game/_CardGame/Blueprints/GamePlay/GI.GI_C|GetPlayerName _gi))
  (Networking|SwitchHasAuthority
    (:Authority
      (Variables|Default|SetUserName _playername))
    (:Remote
      (CallFunction|SetNameRunonServer _playername) ; 轉為伺服器的身分去執行此事件
    )))

(event Custom|SpawnBattleCharacter
  (bind _battle_list (Variables|Default|GetBattle%20List))
  (bind _output (Utilities|Array|Get(acopy) _battle_list))
  (bind (_charactertype _buff) (Utilities|Struct|BreakStruct_CharacterData _output))
  (bind (_普通攻擊_montage _進階攻擊_montage) (CallFunction|GetNPCMontage _charactertype))
  (bind _returnvalue (Game|SpawnActorfromClass (CallFunction|GetNPCClass _charactertype) (Variables|Default|GetBattleCharacterSpawnPotin) "Undefined" (Game|GetPlayerController) _進階攻擊_montage _普通攻擊_montage _buff (PlayerState|GetPawn) (Variables|Default|GetTeam) _charactertype 0))
  (Variables|Default|SetCurrentBattleCharacter _returnvalue)
  (Utilities|Array|RemoveIndex (Variables|Default|GetBattle%20List)))