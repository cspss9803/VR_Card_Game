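; Blueprint function library for the card game, providing shared lookups for framework objects and NPC data.
; Getters return the game state, game mode and game instance already cast to the project's GS, GM and GI classes.
; Two switches on the NPC type map each character to its Blueprint class and to its pair of normal and advanced attack montages.
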(fn GetGS
  (bind _asgs (Utilities|Casting|CastToGS (Game|GetGameState)))
  (return _asgs))

(fn GetGM
  (bind _asgm (Utilities|Casting|CastToGM (Game|GetGameMode)))
  (return _asgm))

(fn GetGI
  (bind _asgi (Utilities|Casting|CastToGI (Game|GetGameInstance)))
  (return _asgi))

(fn GetNPCClass
  (params (NPC_Character :type E_Character%20Enum :default "NewEnumerator0"))
  (switch Utilities|FlowControl|Switch|SwitchonE_Character NPC_Character
    (:NewEnumerator4
      (return "/Game/_AI/NPC_Base/BP_NPC_Lava.BP_NPC_Lava_C"))
    (:NewEnumerator5
      (return "/Game/_AI/NPC_Base/BP_NPC_Man.BP_NPC_Man_C"))
    (:NewEnumerator6
      (return "/Game/_AI/NPC_Base/BP_S_Goblin.BP_S_Goblin_C"))
    (:NewEnumerator7
      (return "/Game/_AI/NPC_Base/BP_NPC_Mutant.BP_NPC_Mutant_C"))
    (:NewEnumerator8
      (return "/Game/_AI/NPC_Base/BP_NPC_Goblin.BP_NPC_Goblin_C"))
    (:NewEnumerator9
      (return "/Game/_AI/NPC_Base/BP_NPC_Forest.BP_NPC_Forest_C"))
    (:NewEnumerator10
      (return "/Game/_AI/NPC_Base/BP_NPC_Beast.BP_NPC_Beast_C"))))

(fn GetNPCMontage
  (params (NPC :type E_Character%20Enum :default "NewEnumerator0"))
  (switch Utilities|FlowControl|Switch|SwitchonE_Character NPC
    (:NewEnumerator4
      (return "/Game/_AI/NPC_Lava/動作/montage/Mutant_Swiping_Montage.Mutant_Swiping_Montage" "/Game/_AI/NPC_Lava/動作/montage/Standing_2H_Magic_Attack_05_Montage.Standing_2H_Magic_Attack_05_Montage"))
    (:NewEnumerator5
      (return "/Game/_AI/NPC_Man/動作/montage/Standing_Melee_Attack_Horizontal_Montage.Standing_Melee_Attack_Horizontal_Montage" "/Game/_AI/NPC_Man/動作/montage/Standing_Melee_Combo_Attack_2_Montage.Standing_Melee_Combo_Attack_2_Montage"))
    (:NewEnumerator6
      (return "/Game/_AI/NPC_S_Goblin/動作/Anim_Assassin_attack1_Montage.Anim_Assassin_attack1_Montage" "/Game/_AI/NPC_S_Goblin/動作/Anim_Assassin_attack1_Montage.Anim_Assassin_attack1_Montage"))
    (:NewEnumerator7
      (return "/Game/_AI/NPC_Mutant/動作/montage/Mutant_Punch_Montage.Mutant_Punch_Montage" "/Game/_AI/NPC_Mutant/動作/montage/Mutant_Punch_Montage.Mutant_Punch_Montage"))
    (:NewEnumerator8
      (return "/Game/_AI/NPC_Goblin/動作/atk_1_Montage.atk_1_Montage" "/Game/_AI/NPC_Goblin/動作/atk_5_Montage.atk_5_Montage"))
    (:NewEnumerator9
      (return "/Game/_AI/NPC_Forest/動作/Attack_01_Seq_Montage.Attack_01_Seq_Montage" "/Game/_AI/NPC_Forest/動作/Attack_09_Begin_Seq_Montage.Attack_09_Begin_Seq_Montage"))
    (:NewEnumerator10
      (return "/Game/_AI/NPC_Beast/動作/Standing_Melee_Attack_Horizontal_Montage.Standing_Melee_Attack_Horizontal_Montage" "/Game/_AI/NPC_Beast/動作/Standing_Melee_Run_Jump_Attack_Montage.Standing_Melee_Run_Jump_Attack_Montage"))))