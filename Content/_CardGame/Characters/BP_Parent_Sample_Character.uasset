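; Parent Blueprint for a card-game sample character, with a color-tinted dissolve effect and an overhead buff list.
; BeginPlay creates the WB_BuffList widget and applies the character's Color to mesh, dissolve edge and particles.
; A Timeline then drives the dissolve amount on both mesh materials and Niagara system.
; Tick turns the widget toward the owning PlayerController's camera, and a custom event passes new Buff data to the list.
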(event Custom|將新的%20Buff%20加到樣本角色頭上的介面
  (params (Buff :type E_Buff%20Enum :default "NewEnumerator4"))
  (bind _aswb_buff_list (Utilities|Casting|CastToWB_BuffList (UserInterface|GetWidget (Variables|Default|GetWidget))))
  (Default|ResetBuffList _aswb_buff_list Buff))

(event EventBeginPlay
  (bind _color (Variables|Default|GetColor))
  (bind _niagarasystemdissolving (Variables|Default|GetNiagaraSystemDissolving))
  (bind _mesh (Variables|Character|GetMesh))
  (bind _returnvalue (Math|Conversions|ToVector(LinearColor) _color))
  (Utilities|FlowControl|Sequence
    (:then_0
      (Class|WidgetComponent|SetDrawSize (Variables|Default|GetWidget) "(X=1500.000000,Y=300.000000)")
      (bind _returnvalue_2 (UserInterface|CreateWidget "/Game/_CardGame/3D_Widget/MainMap/BuffList/WB_BuffList.WB_BuffList_C" 0 self))
      (UserInterface|SetWidget (Variables|Default|GetWidget) _returnvalue_2))
    (:then_1
      (Rendering|Material|SetVectorParameterValueonMaterials (Variables|Character|GetMesh) "Tint" _returnvalue)
      (Utilities|FlowControl|Sequence
        (:then_0
          (Rendering|Material|SetScalarParameterValueonMaterials _mesh "DissolvingAmount" 1.0)
          (Niagara|SetNiagaraVariable(Float) _niagarasystemdissolving "DissolvingAmount" 1.0)
          (bind _tl_animation (Timeline|Timeline Play)
            (:Update
              (Rendering|Material|SetScalarParameterValueonMaterials (Variables|Character|GetMesh) "DissolvingAmount" _tl_animation)
              (Niagara|SetNiagaraVariable(Float) (Variables|Default|GetNiagaraSystemDissolving) "DissolvingAmount" _tl_animation))))
        (:then_1
          (Rendering|Material|SetVectorParameterValueonMaterials _mesh "DissolvingEdgeColor" _returnvalue)
          (Niagara|SetNiagaraVariable(LinearColor) _niagarasystemdissolving "ParitcleColor" (Variables|Default|GetColor)))))))

(event EventTick
  (params (DeltaSeconds :type Float%20%28single-precision%29))
  (bind _widget (Variables|Default|GetWidget))
  (bind _asplayer_controller (Utilities|Casting|CastToPlayerController (Components|GetOwner)))
  (Transformation|SetWorldRotation _widget (Math|Rotator|FindLookatRotation (Transformation|GetWorldLocation _widget) (Camera|GetCameraLocation (Variables|/Script/Engine.PlayerController|GetPlayerCameraManager _asplayer_controller))) false false) ; 設定 Widget 的旋轉值，讓它面向鏡頭
)

(fn ConstructionScript)