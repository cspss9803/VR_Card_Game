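; BP_HomingMissile_Attack is an effect actor for a homing missile attack, built around a Niagara component.
; On BeginPlay it finds a BP_HomingMissile_Target actor and passes that actor's root world location to the Niagara TargetLoaction variable once, with no later updates.
; An unconnected delayed chain would zero the projectile count and then deactivate the effect, but it never runs.
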(event EventBeginPlay
  (bind _returnvalue (Actor|GetActorOfClass "/Game/_CardGame/特效/HomingMissile/BP_HomingMissile_Target.BP_HomingMissile_Target_C"))
  (Niagara|SetNiagaraVariable(Vector3) (Variables|Default|GetNiagara) "TargetLoaction" (Transformation|GetWorldLocation (Variables|/Script/Engine.Actor|GetRootComponent _returnvalue))))

(event Collision|EventActorBeginOverlap
  (params (OtherActor :type Actor%20Object%20Reference)))

(event EventTick
  (params (DeltaSeconds :type Float%20%28single-precision%29)))

(fn ConstructionScript)