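; BP_StaticMesh_Dissolving is an effect actor that repeatedly dissolves and restores a static mesh with accompanying particles.
; On BeginPlay it zeroes the dissolve amount and sets a blue-violet color on both the material edge and the Niagara particles.
; A Timeline drives the DissolvingAmount parameter on the mesh materials and Niagara system together.
; The Timeline ping-pongs endlessly via an AlreadyReverse flag, pausing briefly before each pass.
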(event EventBeginPlay
  (bind _returnvalue (Math|Conversions|ToVector(LinearColor) "(R=0.106177,G=0.000000,B=1.000000,A=1.000000)"))
  (bind _staticmesh (Variables|Default|GetStaticMesh))
  (bind _timeline (Variables|Default|GetTimeline))
  (bind _niagarasystem_dissolving (Variables|Default|GetNiagaraSystem_Dissolving))
  (Utilities|FlowControl|Sequence
    (:then_0
      (Rendering|Material|SetScalarParameterValueonMaterials _staticmesh "DissolvingAmount" 0.0)
      (Niagara|SetNiagaraVariable(Float) _niagarasystem_dissolving "DissolvingAmount" 0.0)
      (Utilities|FlowControl|Delay 1.0)
      (bind _tl_animation (Timeline|Timeline Play)
        (:Update
          (Rendering|Material|SetScalarParameterValueonMaterials (Variables|Default|GetStaticMesh) "DissolvingAmount" _tl_animation)
          (Niagara|SetNiagaraVariable(Float) (Variables|Default|GetNiagaraSystem_Dissolving) "DissolvingAmount" _tl_animation))
        (:Finished
          (if (Variables|Default|GetAlreadyReverse?)
            (Utilities|FlowControl|Delay 1.0)
            (Components|Timeline|PlayfromStart _timeline)
            (Variables|Default|SetAlreadyReverse? false)
            (else
              (Utilities|FlowControl|Delay 1.0)
              (Components|Timeline|ReversefromEnd _timeline)
              (Variables|Default|SetAlreadyReverse? true))))))
    (:then_1
      (Rendering|Material|SetVectorParameterValueonMaterials _staticmesh "DissolvingEdgeColor" _returnvalue)
      (Niagara|SetNiagaraVariable(LinearColor) _niagarasystem_dissolving "ParticleColor" (Math|Conversions|ToLinearColor(Vector) _returnvalue)))))

(fn ConstructionScript)