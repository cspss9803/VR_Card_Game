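; BP_Crystal is a team-colored crystal actor in the card game that dissolves into view on spawn and back out when destroyed.
; BeginPlay picks the red or blue material and color by Team, then starts the dissolve timeline after an Index-based delay, staggering crystals.
; The timeline drives both the mesh material's dissolve parameter and a Niagara particle system.
; DestroyCrystal reverses the timeline, then destroys the actor once it finishes.
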(event Custom|DestroyCrystal
  (bind _timeline (Variables|Default|GetTimeline))
  (Components|Timeline|ReversefromEnd _timeline)
  (Utilities|FlowControl|Delay (+ (Components|Timeline|GetTimelineLength _timeline) 1.0))
  (Actor|DestroyActor))

(event EventBeginPlay
  (bind _staticmesh (Variables|Default|GetStaticMesh))
  (bind _niagarasystem_dissolving (Variables|Default|GetNiagaraSystem_Dissolving))
  (bind _staticmesh_2 (Variables|Default|GetStaticMesh))
  (switch Utilities|FlowControl|Switch|SwitchonE_Team (Variables|Default|GetTeam)
    (:NewEnumerator1
      (Variables|Default|SetColor (Math|Conversions|ToVector(LinearColor) "(R=2.000000,G=0.000000,B=0.018016,A=1.000000)"))
      (Rendering|Material|SetMaterial _staticmesh_2 0 "/Game/_CardGame/靜態模型/Crystal/MI_Crystal_Red.MI_Crystal_Red"))
    (:NewEnumerator2
      (Variables|Default|SetColor (Math|Conversions|ToVector(LinearColor) "(R=0.000000,G=0.199559,B=2.000000,A=1.000000)"))
      (Rendering|Material|SetMaterial _staticmesh_2 0 "/Game/_CardGame/靜態模型/Crystal/MI_Crystal_Blue.MI_Crystal_Blue")))
  (Utilities|FlowControl|Sequence
    (:then_0
      (Rendering|Material|SetScalarParameterValueonMaterials _staticmesh "DissolvingAmount" 1.0)
      (Niagara|SetNiagaraVariable(Float) _niagarasystem_dissolving "DissolvingAmount" 1.0)
      (Niagara|SetNiagaraVariable(Float) _niagarasystem_dissolving "ParticleAmount" 1e+04))
    (:then_1
      (Rendering|Material|SetVectorParameterValueonMaterials _staticmesh "DissolvingEdgeColor" (Variables|Default|GetColor))
      (Niagara|SetNiagaraVariable(LinearColor) _niagarasystem_dissolving "ParticleColor" (Math|Conversions|ToLinearColor(Vector) (Variables|Default|GetColor))))
    (:then_2
      (Utilities|FlowControl|Delay (+ (* (Variables|Default|Getindex) 0.5) 1.0))
      (bind _tl_animation (Timeline|Timeline Play)
        (:Update
          (Rendering|Material|SetScalarParameterValueonMaterials (Variables|Default|GetStaticMesh) "DissolvingAmount" _tl_animation)
          (Niagara|SetNiagaraVariable(Float) (Variables|Default|GetNiagaraSystem_Dissolving) "DissolvingAmount" _tl_animation))))))

(fn ConstructionScript)