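; BP_NPC_Display is a sample NPC character that shows one NPC type with a buff list widget above its head.
; BeginPlay picks skeletal mesh and anim class by type, creates WB_BuffList, and applies the type's color to tint, dissolve edge and particles.
; A timeline drives the dissolve amount on both materials and Niagara.
; Tick turns the widget toward the owning PlayerController's camera, and a custom event passes new buffs to the list.
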(event Custom|將新的%20Buff%20加到樣本角色頭上的介面
  (params (Buff :type E_Buff%20Enum :default "NewEnumerator4"))
  (bind _aswb_buff_list (Utilities|Casting|CastToWB_BuffList (UserInterface|GetWidget (Variables|Default|GetWidget))))
  (Default|ResetBuffList _aswb_buff_list Buff))

(event EventBeginPlay
  (bind _npc_種類 (Variables|Default|GetNPC%20種類))
  (bind _niagarasystemdissolving (Variables|Default|GetNiagaraSystemDissolving))
  (bind _mesh (Variables|Character|GetMesh))
  (bind _顏色 (CallFunction|取得NPC的顏色 _npc_種類))
  (bind _returnvalue (Math|Conversions|ToVector(LinearColor) _顏色))
  (Components|SkeletalMesh|SetSkeletalMeshAsset (Variables|Character|GetMesh) (CallFunction|取得NPC的骨骼模型 (Variables|Default|GetNPC%20種類)))
  (Class|SkeletalMeshComponent|SetAnimClass (Variables|Character|GetMesh) (CallFunction|取得NPC的動畫藍圖類別 (Variables|Default|GetNPC%20種類)))
  (Utilities|FlowControl|Sequence
    (:then_0
      (Class|WidgetComponent|SetDrawSize (Variables|Default|GetWidget) "(X=1500.000000,Y=300.000000)")
      (bind _returnvalue_2 (UserInterface|CreateWidget "/Game/_Waraces/Cards/Card_UIs/BuffList/WB_BuffList.WB_BuffList_C" 0 self))
      (UserInterface|SetWidget (Variables|Default|GetWidget) _returnvalue_2))
    (:then_1
      ;[1 1 1] Comment
      (Rendering|Material|SetVectorParameterValueonMaterials (Variables|Character|GetMesh) "Tint" _returnvalue)
      (Utilities|FlowControl|Sequence
        (:then_0
          (Rendering|Material|SetScalarParameterValueonMaterials _mesh "DissolvingAmount" 1.0)
          (Niagara|SetNiagaraVariable(Float) _niagarasystemdissolving "DissolvingAmount" 1.0)
          (bind _tl_animation (Timeline|Timeline Play)
            (:Update
              (Rendering|Material|SetScalarParameterValueonMaterials (Variables|Character|GetMesh) "DissolvingAmount" _tl_animation)
              (Niagara|SetNiagaraVariable(Float) (Variables|Default|GetNiagaraSystemDissolving) "DissolvingAmount" _tl_animation))))
        (:then_1
          (Rendering|Material|SetVectorParameterValueonMaterials _mesh "DissolvingEdgeColor" _returnvalue)
          (Niagara|SetNiagaraVariable(LinearColor) _niagarasystemdissolving "ParitcleColor" _顏色))))))

(event EventTick
  (params (DeltaSeconds :type Float%20%28single-precision%29))
  (bind _widget (Variables|Default|GetWidget))
  (bind _asplayer_controller (Utilities|Casting|CastToPlayerController (Components|GetOwner)))
  (Transformation|SetWorldRotation _widget (Math|Rotator|FindLookatRotation (Transformation|GetWorldLocation _widget) (Camera|GetCameraLocation (Variables|/Script/Engine.PlayerController|GetPlayerCameraManager _asplayer_controller))) false false) ; 設定 Widget 的旋轉值，讓它面向鏡頭
)

(fn ConstructionScript)

(fn 取得NPC的骨骼模型
  (params (NPC :type E_NPC%20Enum :default "NewEnumerator0"))
  (switch Utilities|FlowControl|Switch|SwitchonE_NPC NPC
    (:NewEnumerator0
      (return 0))
    (:NewEnumerator4
      (return "/Game/_Waraces/AI_Charcaters/NPC_Lava/Meshes/SK_Lava.SK_Lava"))
    (:NewEnumerator6
      (return "/Game/_Waraces/AI_Charcaters/NPC_S_Goblin/Meshes/SK_S_Goblin.SK_S_Goblin"))
    (:NewEnumerator8
      (return "/Game/_Waraces/AI_Charcaters/NPC_Goblin/Meshes/SK_Goblin.SK_Goblin"))
    (:NewEnumerator9
      (return "/Game/_Waraces/AI_Charcaters/NPC_Forest/Meshes/SK_Forest.SK_Forest"))
    (:NewEnumerator10
      (return "/Game/_Waraces/AI_Charcaters/NPC_Beast/Meshes/SK_Beast.SK_Beast"))
    (:NewEnumerator11
      (return "/Game/_Waraces/AI_Charcaters/NPC_SpearMan/Meshes/SK_SpearMan.SK_SpearMan"))
    (:NewEnumerator12
      (return "/Game/_Waraces/AI_Charcaters/NPC_Human/Meshes/SK_Human.SK_Human"))))

(fn 取得NPC的動畫藍圖類別
  (params (NPC :type E_NPC%20Enum :default "NewEnumerator0"))
  (switch Utilities|FlowControl|Switch|SwitchonE_NPC NPC
    (:NewEnumerator0
      (return 0))
    (:NewEnumerator4
      (return "/Game/_Waraces/AI_Charcaters/NPC_Lava/Animations/ABP_Lava.ABP_Lava_C"))
    (:NewEnumerator6
      (return "/Game/_Waraces/AI_Charcaters/NPC_S_Goblin/Animations/ABP_S_Goblin.ABP_S_Goblin_C"))
    (:NewEnumerator8
      (return "/Game/_Waraces/AI_Charcaters/NPC_Goblin/Animations/ABP_Goblin.ABP_Goblin_C"))
    (:NewEnumerator9
      (return "/Game/_Waraces/AI_Charcaters/NPC_Forest/Animations/ABP_Forest.ABP_Forest_C"))
    (:NewEnumerator10
      (return "/Game/_Waraces/AI_Charcaters/NPC_Beast/Animations/ABP_Beast.ABP_Beast_C"))
    (:NewEnumerator11
      (return "/Game/_Waraces/AI_Charcaters/NPC_SpearMan/Animations/ABP_SpearMan.ABP_SpearMan_C"))
    (:NewEnumerator12
      (return "/Game/_Waraces/AI_Charcaters/NPC_Human/Animations/ABP_Human.ABP_Human_C"))))