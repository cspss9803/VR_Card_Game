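; Spearman NPC Blueprint that extends a parent NPC class with spear-specific attacks and weapon attachment points.
; On BeginPlay it assigns thrust and turn-then-lying montages as the normal and advanced attacks, then runs the parent logic.
; Override-style functions supply the weapon mesh's hand_l socket location in RightHand bone space, as used for two-handed grips, and its launch-position socket transform.
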(event EventBeginPlay
  (Variables|Default|Set普通攻擊_Montage "/Game/_Waraces/AI_Charcaters/NPC_SpearMan/Animations/AM_SpearMan_Attack_Thrust.AM_SpearMan_Attack_Thrust")
  (Variables|Default|Set進階攻擊_Montage "/Game/_Waraces/AI_Charcaters/NPC_SpearMan/Animations/AM_SpearMan_Attack_Turn_Then_Lying.AM_SpearMan_Attack_Turn_Then_Lying")
  (|CallParentFunction))

(event Collision|EventActorBeginOverlap
  (params (OtherActor :type Actor%20Object%20Reference)))

(event EventTick
  (params (DeltaSeconds :type Float%20%28single-precision%29)))

(fn ConstructionScript
  (|CallParentFunction))

(fn FWeaponTransform
  (bind _staticmesh (Variables|Default|GetStaticMesh))
  (Utilities|IsValid _staticmesh
    (:Is%20Valid
      (return (Math|Transform|MakeTransform (.OutPosition (Class|SkinnedMeshComponent|TransformtoBoneSpace (Variables|Character|GetMesh) "RightHand" (.location (Transformation|GetSocketTransform _staticmesh "hand_l" "RTS_World")) "0, 0, 0")) "0, 0, 0" "1.000000,1.000000,1.000000")))))

(fn FGet發射位置
  (bind _staticmesh (Variables|Default|GetStaticMesh))
  (Utilities|IsValid _staticmesh
    (:Is%20Valid
      (return (Transformation|GetSocketTransform _staticmesh "發射位置" "RTS_World")))))