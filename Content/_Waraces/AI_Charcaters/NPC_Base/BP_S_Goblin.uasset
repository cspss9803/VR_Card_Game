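; BP_S_Goblin is a short-lived small goblin NPC that dies automatically nine seconds after spawning.
; BeginPlay registers its dagger for the dissolve effect, runs the parent logic and sets its walk speeds.
; After the delay, the server stops its attack by switching the AI controller to an empty behavior tree, then triggers death.
; A separate event disables its damage by zeroing attack power.
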(event Custom|小哥布林停止攻擊
  (bind _asnpc_aicontroller (Utilities|Casting|CastToNPC_AIcontroller (Pawn|GetController)))
  (AI|RunBehaviorTree _asnpc_aicontroller "/Game/_Waraces/AI_Charcaters/_AI/Behavior_Tree/BP_Empty.BP_Empty"))

(event Custom|不允許小哥布林造成傷害
  (Variables|Default|Set目前攻擊力 0.0))

(event EventBeginPlay
  (bind _charactermovement (Variables|Character|GetCharacterMovement))
  (Variables|Default|Set所有需要消散特效的靜態模型 (Utilities|Array|MakeArray (Variables|Default|Get匕首)))
  (|CallParentFunction)
  (Variables|/Script/Engine.CharacterMovementComponent|SetMaxWalkSpeed _charactermovement 2e+02)
  (Variables|/Script/Engine.CharacterMovementComponent|SetMaxWalkSpeedCrouched _charactermovement 2e+02)
  (Utilities|FlowControl|Delay 9.0)
  (Networking|SwitchHasAuthority
    (:Authority
      (CallFunction|小哥布林停止攻擊)
      (CallFunction|死亡))))

(fn ConstructionScript
  (|CallParentFunction))