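; Lightning-strike area-of-effect Blueprint in the Goblin NPC VFX folder, named and commented as a damage-over-time effect.
; It overrides Trigger to call the parent, then attach the NS_PurpleStrike effect to its root and play the second-skill sound at the actor's location.
; It contains no damage logic of its own; BeginPlay, overlap and Tick are disabled stubs, and the construction script only calls the parent.
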(event EventBeginPlay
  (|CallParentFunction) ; This node is disabled and will not be called.\nDrag off pins to build functionality.
)

(event Collision|EventActorBeginOverlap
  (params (OtherActor :type Actor%20Object%20Reference))
  (|CallParentFunction OtherActor) ; This node is disabled and will not be called.\nDrag off pins to build functionality.
)

(event EventTick
  (params (DeltaSeconds :type Float%20%28single-precision%29))
  (|CallParentFunction DeltaSeconds) ; This node is disabled and will not be called.\nDrag off pins to build functionality.
)

(event EventTrigger
  (|CallParentFunction)
  (Niagara|SpawnSystemAttached "/Game/_Waraces/AI_Charcaters/NPC_Goblin/VFXs/StylizedVFX-AirStrikes/NS_PurpleStrike.NS_PurpleStrike" (Variables|Default|GetDefaultSceneRoot) "None" "0, 0, 0" "0, 0, 0" "KeepRelativeOffset" false)
  (Audio|PlaySoundatLocation "/Game/_Waraces/AI_Charcaters/NPC_Goblin/Audio/第二招音效.第二招音效" (Transformation|GetActorLocation self) "0, 0, 0" 1.0 1.0 0.0 0 0 0 0))

(fn ConstructionScript
  (|CallParentFunction))