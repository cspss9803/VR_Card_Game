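; Game Instance for the VR game, handling LAN hosting and joining, direct IP connection, tutorial launch and quitting.
; Each event drives the passed-in headset message widget's transition mask and status text, restoring start-menu options when search or join fails.
; Hosting opens the main map as a two-player listen server; IP connection uses the "open" console command with a fixed-delay failure message.
; It also spawns a 3D virtual keyboard near the VR pawn for text fields.
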(event Custom|IP%20連線
  (params (IP :type Text) (頭顯訊息介面 :type WB%20HMD%20Object%20Reference))
  (Default|顯示過場遮罩 頭顯訊息介面 "正在連線到此IP...")
  (|進行IP連線 IP)
  (Utilities|FlowControl|Delay 1e+01)
  (Default|隱藏過場遮罩 頭顯訊息介面 "無法連線到此IP" 1.0))

(event Custom|創建房間
  (params (頭顯訊息介面 :type WB%20HMD%20Object%20Reference))
  (Default|顯示過場遮罩 頭顯訊息介面 "創建中...")
  (Utilities|FlowControl|Delay 1.0)
  (|Session (Game|GetPlayerController 0) 2 true
    (:OnSuccess
      (Game|OpenLevel(byObjectReference) "/Game/_Waraces/Maps/Map_主場景.Map_主場景" true "?Listen"))
    (:OnFailure
      (Default|隱藏過場遮罩 頭顯訊息介面 "創建時發生錯誤" 1.0))))

(event Custom|關閉遊戲
  (params (頭顯訊息介面 :type WB%20HMD%20Object%20Reference))
  (Default|顯示過場遮罩 頭顯訊息介面 "正在關閉...")
  (Utilities|FlowControl|Delay 1.0)
  (Game|QuitGame (Game|GetPlayerController 0) "Quit" false))

(event Custom|加入房間
  (params (頭顯訊息介面 :type WB%20HMD%20Object%20Reference))
  (Default|顯示過場遮罩 頭顯訊息介面 "尋找中...")
  (bind _搜尋結果 (|CollapseGraph)
    (:有找到房間
      (Default|設定系統訊息 頭顯訊息介面 "連線中...")
      (Utilities|FlowControl|Delay 1.0)
      (|加入房間 _搜尋結果
        (:OnSuccess
          (Default|設定系統訊息 頭顯訊息介面 "連線成功，正加加入房間"))
        (:OnFailure
          (Default|隱藏過場遮罩 頭顯訊息介面 "連線時發生錯誤" 1.0)
          (bind _returnvalue (Actor|GetActorOfClass "/Game/_Waraces/Scene_UIs/StartMap/BP_StartMenu_Manager.BP_StartMenu_Manager_C" :!label _label))
          (Default|淡入所有選項 _returnvalue))))
    (:沒找到房間
      (Default|隱藏過場遮罩 頭顯訊息介面 "沒找到任何房間" 1.0)
      (goto _label))
    (:發生錯誤
      (Default|隱藏過場遮罩 頭顯訊息介面 "尋找時發生錯誤" 1.0)
      (goto _label))))

(event Custom|開始新手導覽
  (params (頭顯訊息介面 :type WB%20HMD%20Object%20Reference))
  (Default|顯示過場遮罩 頭顯訊息介面 "正在前往新手導覽...")
  (Utilities|FlowControl|Delay 1.0)
  (Game|OpenLevel(byObjectReference) "/Game/_Waraces/Maps/Map_教學導覽.Map_教學導覽"))

(fn 生成虛擬鍵盤
  (params (要輸入文字的輸入框 :type Editable%20Text%20Object%20Reference) (覆蓋在輸入框上用來觸發輸入的按鈕 :type Button%20Object%20Reference))
  (bind _asvr_pawn_base (Utilities|Casting|CastToVR_Pawn_Base (Game|Player|GetPlayerPawn 0)))
  (bind _returnvalue (Game|SpawnActorfromClass "/Game/_Waraces/Scene_UIs/StartMap/Keyboard/Actor_3D_Widget_Keyboard.Actor_3D_Widget_Keyboard_C" (Math|Transform|MakeTransform (+ (Math|Vector|MakeVector (.x (Transformation|GetWorldLocation (Variables|/Game/_Waraces/Player/Blueprints/VR_Pawn_Base.VR_Pawn_Base_C|Get相機 _asvr_pawn_base))) (.y (Transformation|GetWorldLocation (Variables|/Game/_Waraces/Player/Blueprints/VR_Pawn_Base.VR_Pawn_Base_C|Get相機 _asvr_pawn_base))) (- (.z (Transformation|GetWorldLocation (Variables|/Game/_Waraces/Player/Blueprints/VR_Pawn_Base.VR_Pawn_Base_C|Get相機 _asvr_pawn_base))) 2e+01)) (* (Transformation|GetActorForwardVector _asvr_pawn_base) 8e+01)) "-30.000000,0.000000,0.000000" "1.000000,1.000000,1.000000") "Undefined" (Game|GetPlayerController 0) 要輸入文字的輸入框 覆蓋在輸入框上用來觸發輸入的按鈕 0))
  (return _returnvalue))