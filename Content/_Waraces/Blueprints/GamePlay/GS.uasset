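; Game State for a multiplayer VR card battler, cycling rounds through character arrangement, buffs, spawning, fights, victory checks, crystal destruction, reset and game over.
; GameStage's OnRep runs each phase's pawn, widget and spawn logic, while server countdowns are meant to advance the stage.
; Three battle wins cost the loser an HP crystal; zero crystals ends the game with fireworks.
; Phases mix VRPawn_Main and VRPawn_Main_old casts.
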(fn ConstructionScript)

(fn OnRepAllPlayerState
  ;[1 1 1] 更新記分板
  (bind _returnvalue (Actor|GetActorOfClass "/Game/_Waraces/Scene_UIs/MainMap/PlayerList/Actor_3D_Widget_PlayerList.Actor_3D_Widget_PlayerList_C"))
  (Default|UpdatePlayerList _returnvalue))

(fn OnRepGameStage
  (switch Utilities|FlowControl|Switch|SwitchonE_GameStage (Variables|Default|GetGameStage)
    (:NewEnumerator1
      (|角色安排階段 1e+01))
    (:NewEnumerator2
      (|增益添加階段 3e+01))
    (:NewEnumerator3
      (|對戰角色生成階段 1.0))
    (:NewEnumerator4
      (|對戰階段))
    (:NewEnumerator5
      (|獲勝檢查階段 1.0))
    (:NewEnumerator7
      (|生命水晶破壞階段))
    (:NewEnumerator6
      (|重設 2.0))
    (:NewEnumerator8
      (|遊戲結束))))

(fn GetVRPawn
  (bind _asvrpawn_main_old (Utilities|Casting|CastToVRPawn_Main_old (Game|Player|GetPlayerPawn 0)))
  (return _asvrpawn_main_old))

(event Custom|LaunchPlayerTimer
  (params (time :type Float%20%28double-precision%29))
  (bind _returnvalue (Actor|GetActorOfClass "/Game/_Waraces/Scene_UIs/MainMap/Timer/Actor_3D_Widget_Timer.Actor_3D_Widget_Timer_C"))
  (Default|LaunchPlayerTimer _returnvalue time (Variables|Default|GetServerTimerLauchTimePoint)))

(event Custom|LaunchTimer
  (params (Time :type Float%20%28double-precision%29) (Only%20Launch%20Server%20Timer? :type Boolean))
  (if (Networking|IsServer)
    (CallFunction|LaunchServerTimer Time)
    (if (not Only%20Launch%20Server%20Timer?)
      (CallFunction|LaunchPlayerTimer Time :!label _label))
    (else
      (goto _label))))

(event Custom|PlayerAmountChange
  (Variables|Default|SetAllPlayerState (Variables|Default|GetPlayerArray)))

(event Custom|ServerCountDown
  (bind _result (Math|Float|DecrementFloat (Variables|Default|GetServerCountDownTime))
    (:%20%20
      (if (not (> _result 0.0))
        (Utilities|Time|ClearandInvalidateTimerbyHandle (Variables|Default|GetServerTimer))
        (return)))))

(event Custom|LaunchServerTimer
  (params (Time :type Float%20%28double-precision%29))
  (Variables|Default|SetServerCountDownTime Time)
  (Variables|Default|SetServerTimerLauchTimePoint (GameState|GetServerWorldTimeSeconds))
  (bind _returnvalue (Utilities|Time|SetTimerbyEvent (delegate Custom|ServerCountDown) 1.0 true))
  (Variables|Default|SetServerTimer _returnvalue))