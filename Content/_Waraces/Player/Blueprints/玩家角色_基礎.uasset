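; Base VR player character that sets up the headset and drives laser-style UI interaction with both hands.
; On BeginPlay, if an HMD is enabled, it sets Stage tracking origin, issues the pixel density console command and adds the IMC_VR Enhanced Input context.
; Left and right trigger actions press and release each hand's widget interactor as a left click, changing its debug color.
; Hover changes play a haptic pulse on the matching hand.
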(event OnHoveredWidgetChanged(介面互動器-右)
  (params (WidgetComponent :type Widget%20Component%20Object%20Reference) (PreviousWidgetComponent :type Widget%20Component%20Object%20Reference))
  (Class|PlayerController|PlayHapticEffect (Game|GetPlayerController 0) "/Game/_Waraces/Player/Haptic_Effect/HapticEffect_Hover.HapticEffect_Hover" "Right" 1.0 false) ; 發出輕震動
)

(event OnHoveredWidgetChanged(介面互動器-左)
  (params (WidgetComponent :type Widget%20Component%20Object%20Reference) (PreviousWidgetComponent :type Widget%20Component%20Object%20Reference))
  (Class|PlayerController|PlayHapticEffect (Game|GetPlayerController 0) "/Game/_Waraces/Player/Haptic_Effect/HapticEffect_Hover.HapticEffect_Hover" "Left" 1.0 false) ; 發出輕震動
)

(event Input|EnhancedActionEvents|EnhancedInputActionIA_Click_Right
  (params (ActionValue :type Boolean) (ElapsedSeconds :type Float%20%28double-precision%29) (TriggeredSeconds :type Float%20%28double-precision%29) (InputAction :type Input%20Action%20Object%20Reference :default "/Game/_Waraces/Player/Inputs/IA_Click_Right.IA_Click_Right"))
  (bind _介面互動器_右 (Variables|Default|Get介面互動器-右))
  (:Started
    (Class|WidgetInteractionComponent|PressPointerKey _介面互動器_右 "LeftMouseButton")
    (Variables|/Script/UMG.WidgetInteractionComponent|SetDebugColor _介面互動器_右 ""))
  (:Completed
    (Class|WidgetInteractionComponent|ReleasePointerKey _介面互動器_右 "LeftMouseButton")
    (Variables|/Script/UMG.WidgetInteractionComponent|SetDebugColor _介面互動器_右 "(R=1.000000,G=1.000000,B=1.000000,A=1.000000)")))

(event Input|EnhancedActionEvents|EnhancedInputActionIA_Click_Left
  (params (ActionValue :type Boolean) (ElapsedSeconds :type Float%20%28double-precision%29) (TriggeredSeconds :type Float%20%28double-precision%29) (InputAction :type Input%20Action%20Object%20Reference :default "/Game/_Waraces/Player/Inputs/IA_Click_Left.IA_Click_Left"))
  (bind _介面互動器_左 (Variables|Default|Get介面互動器-左))
  (:Triggered
    (Class|WidgetInteractionComponent|PressPointerKey _介面互動器_左 "LeftMouseButton")
    (Variables|/Script/UMG.WidgetInteractionComponent|SetDebugColor _介面互動器_左 "(R=1.000000,G=0.960876,B=0.000000,A=1.000000)"))
  (:Completed
    (Class|WidgetInteractionComponent|ReleasePointerKey _介面互動器_左 "LeftMouseButton")
    (Variables|/Script/UMG.WidgetInteractionComponent|SetDebugColor _介面互動器_左 "(R=1.000000,G=1.000000,B=1.000000,A=1.000000)")))

(event EventBeginPlay
  (Utilities|是否啟用了虛擬實境設備?
    (:已啟用
      (|設定VR裝置追蹤位置的基準點)
      (|設定顯示器的像素密度)
      (|設定映射輸入))))

(fn ConstructionScript)