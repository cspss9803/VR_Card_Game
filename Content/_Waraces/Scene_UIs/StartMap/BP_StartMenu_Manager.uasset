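; BP_StartMenu_Manager manages the start menu's four child-actor buttons: create room, join room, rename and quit game.
; On BeginPlay it passes the player character (玩家角色) to each button's WB_Button widget, reached through its WidgetComponent.
; The fade-in-all-options event (淡入所有選項) calls ScaleFadeInAllButton on the create-room button only.
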(event Custom|淡入所有選項
  (bind _asbp_start_menu_button (Utilities|Casting|CastToBP_StartMenu_Button (Variables|/Script/Engine.ChildActorComponent|GetChildActor (Variables|Default|GetButton_創建房間))))
  (Default|ScaleFadeinAllButton _asbp_start_menu_button))

(event EventBeginPlay
  (for _array_element (Utilities|Array|MakeArray (Variables|Default|GetButton_創建房間) (Variables|Default|GetButton_加入房間) (Variables|Default|GetButton_重新命名) (Variables|Default|GetButton_離開遊戲))
    (bind _asbp_start_menu_button (Utilities|Casting|CastToBP_StartMenu_Button (Variables|/Script/Engine.ChildActorComponent|GetChildActor _array_element)))
    (bind _aswb_button (Utilities|Casting|CastToWB_Button (UserInterface|GetWidget (Variables|/Game/_Waraces/Scene_UIs/StartMap/Button/BP_StartMenu_Button.BP_StartMenu_Button_C|GetWidgetComponent_Button _asbp_start_menu_button))))
    (Variables|/Game/_Waraces/Scene_UIs/StartMap/Button/WB_Button.WB_Button_C|Set玩家角色 _aswb_button (Variables|Default|Get玩家角色))))

(fn ConstructionScript)